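; Timer actor that shows a minutes:seconds countdown on a TextRender component in the world.
; On BeginPlay it plays a Timeline in reverse from the end, using the track value as seconds remaining.
; Each update derives minutes by flooring and seconds by scaling the fraction and slicing two decimal digits from its string, showing "60" as "00".
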(event EventBeginPlay
  ;[1 1 1] Время в секундах. Во втором узле значение и time должны быть равными, тогда скорость будет ок.
  (bind _newtrack_0 (Timeline|Timeline_0 ReverseFromEnd)
    (:Update
      (Variables|Default|SetMin (Math|Float|Floor (/ _newtrack_0 6e+01)))
      (Variables|Default|SetSec (Math|Float|Fraction (/ _newtrack_0 6e+01)))
      (if (Utilities|Enum|Equal(Enum) (Class|KismetStringLibrary|Mid (Utilities|String|ToString(Float) (/ (Variables|Default|GetSec) 1.67)) 2 2) "60")
        (Variables|Default|SetTimerString "00")
        (else
          (Variables|Default|SetTimerString (Class|KismetStringLibrary|Mid (Utilities|String|ToString(Float) (/ (Variables|Default|GetSec) 1.67)) 2 2))))
      (Rendering|Components|TextRender|SetText (Variables|Default|GetTextRender) (Utilities|Text|ToText(String) (Utilities|String|Append (Utilities|String|ToString(Integer) (Variables|Default|GetMin)) (Utilities|String|Append ":" (Variables|Default|GetTimerString))))))))

(fn ConstructionScript)